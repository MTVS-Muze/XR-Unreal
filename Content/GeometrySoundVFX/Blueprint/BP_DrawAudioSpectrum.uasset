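; Audio visualizer actor that plays three songs in a loop and draws their spectrum into a render target.
; On playback progress, it samples offline AudioSynesthesia Constant-Q data at the current time, drawing each band as a grayscale cell in an XY grid, scaled by sensitivity.
; Tick spins and bobs the visualization models.
; UI mode adds a sensitivity slider and a dropdown choosing the visible model; otherwise all models are hidden.
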(event `self.ReceiveBeginPlay`
  (bind _uiwidget (`self.UIWidget`))
  (if (`self.UIMode`)
    ;[1 1 1] Create UI widget and Bind Events
    (bind _returnvalue (`|CreateWidget` "/Game/GeometrySoundVFX/Blueprint/WBP/WBP_UI.WBP_UI_C"))
    (bind _output_get (set `self.UIWidget` _returnvalue))
    (`UserWidget.AddToViewport` _output_get 0)
    (add `Slider.OnValueChanged` (`/Game/GeometrySoundVFX/Blueprint/WBP/WBP_UI.Handle_Sensitivity` _uiwidget) (delegate `Slide_Sensitivity`))
    (add `ComboBoxString.OnSelectionChanged` (`/Game/GeometrySoundVFX/Blueprint/WBP/WBP_UI.ComboBox_VisualizationStyle` _uiwidget) (delegate `DropdownBox_VisualizationStyle`))
    ;[1 1 1] Set Input Mode as UI Only
    (`WidgetBlueprintLibrary.SetInputMode_UIOnlyEx` null null)
    (set `PlayerController.bShowMouseCursor` true (`GameplayStatics.GetPlayerController` 0)))
  ;[1 1 1] Initialize Render Target Canvas ( RT_SpectrumTexture )
  (`KismetRenderingLibrary.ClearRenderTarget2D` (`self.RenderTargetTexture`))
  (`self.CreateRT`)
  ;[1 1 1] Set and Play Sound
  (`self.PlaySound` (`self.SoundWav`))
  ;[1 1 1] Create Model Array
  (bind _output_get_2 (set `self.ModelArray` (`|MakeArray` (`self.Cube`) (`self.Cube2`) (`self.Cube3`) (`self.Circular`) (`self.Circular2`) (`self.Circular3`) (`self.HexGrid`) (`self.HexGrid2`) (`self.HexGrid3`) (`self.HexSphere`) (`self.HexSphere2`) (`self.HexSphere3`) (`self.HexSphere4`) (`self.NoiseWave`) (`self.NoiseWave2`) (`self.NoiseWave3`) (`self.NoiseWave4`) (`self.NoiseWave5`) (`self.NoiseWave6`) (`self.NoiseWave7`) (`self.NoiseWave8`) (`self.NoiseWave9`) (`self.NoiseWave10`) (`self.NoiseWave11`) (`self.NoiseWave12`))))
  (if (`self.UIMode`)
    ;[1 1 1] Set Model Visibility
    (`self.ModelVisibility` _output_get_2)
    (`AudioComponent.AdjustVolume` (`self.Audio`) 0.0 0.01 "Linear")
    (else
      (for _array_element (`self.ModelArray`)
        (`SceneComponent.SetVisibility` _array_element false false)))))

(event `Slide_Sensitivity`
  (params (Value :type "Float (single-precision)"))
  ;[1 1 1] Set Sensitivity For Sound Visualization
  (set `self.SoundSensitivity` (* (`KismetMathLibrary.MapRangeUnclamped` Value 0.0 1.0 0.2 1.0) 2.0)))

(event `DropdownBox_VisualizationStyle`
  (params (SelectedItem :type String) (SelectionType :type "ESelectInfo Enum" :default "OnKeyPress"))
  ;[1 1 1] Dropdown Box For Setting Visibility of Models
  (set `self.ModelIndex` (`ComboBoxString.GetSelectedIndex` (`/Game/GeometrySoundVFX/Blueprint/WBP/WBP_UI.ComboBox_VisualizationStyle` (`self.UIWidget`))))
  (`self.ModelVisibility` (`self.ModelArray`)))

(event `self.Audio.OnAudioPlaybackPercent`
  (params (PlayingSoundWave :type "SoundWave Object Reference") (PlaybackPercent :type "Float (single-precision)"))
  (bind _pixelsize (`self.PixelSize`))
  ;[1 1 1] When Music Finished
  (if (== PlaybackPercent 1.0)
    ;[1 1 1] Play Next Music
    (`/Engine/EditorBlueprintResources/StandardMacros.IncrementInt` (`self.MusisIndex`)
      (:`  `
        (if (not (<= (`self.MusisIndex`) 2))
          (set `self.MusisIndex` 0))
        (switch `int` (`self.MusisIndex`)
          (:`Default`
            (`self.PlaySound` (`self.SoundWav`) :!label _label)
            (set `self.Target` "/Game/GeometrySoundVFX/Blueprint/SNRT_AudioSynesthesiaNRT.SNRT_AudioSynesthesiaNRT"))
          (:`0`
            (goto _label))
          (:`1`
            (`self.PlaySound` (`self.SoundWav2`))
            (set `self.Target` "/Game/GeometrySoundVFX/Blueprint/SNRT_AudioSynesthesiaNRT2.SNRT_AudioSynesthesiaNRT2"))
          (:`2`
            (`self.PlaySound` (`self.SoundWav3`))
            (set `self.Target` "/Game/GeometrySoundVFX/Blueprint/SNRT_AudioSynesthesiaNRT3.SNRT_AudioSynesthesiaNRT3")))))
    (else
      ;[1 1 1] Calculate Current Timeline in Seconds
      (set `self.MusicTimeline` (* (`self.MusicDuration`) PlaybackPercent))
      ;[1 1 1] Draw Render Target Texture From Audio Spectrum
      (for (_array_element _array_index) (`self.XYMatrixArray`)
        (`self.DrawRT` _array_element (`KismetMathLibrary.MakeVector2D` _pixelsize _pixelsize) (* (`|GetArrayItem` (`ConstantQNRT.GetNormalizedChannelConstantQAtTime` (`self.Target`) (`self.MusicTimeline`) 0) _array_index) (`self.SoundSensitivity`)))))))

(event `self.ReceiveTick`
  (params (DeltaSeconds :type "Float (single-precision)"))
  (bind _modelarray (`self.ModelArray`))
  ;[1 1 1] Rotation and Up&Down Animation
  (`SceneComponent.K2_AddRelativeRotation` _modelarray (`KismetMathLibrary.MakeRotator` 0.0 0.0 (* DeltaSeconds 50.0)) false false)
  (`SceneComponent.K2_AddRelativeLocation` _modelarray (`KismetMathLibrary.MakeVector` 0.0 0.0 (* (`KismetMathLibrary.Sin` (* (`GameplayStatics.GetTimeSeconds`) 2.0)) 0.1)) false false))

(fn `CreateRT`
  (bind _pixelsize (`self.PixelSize`))
  (bind _pixelsize_2 (`self.PixelSize`))
  (bind _returnvalue (* (`self.XNum`) (`self.YNum`)))
  ;[1 1 1] Make Pixel Matrix of Render Target Texture ( X * Y ) and Initialize it
  ;;[1 1 1] ex) For creating 8 x 8 matrix in Rentarget Texture,
  ;; Size X (RenderTarget) / XNum = Pixel Size
  ;; 1024 / 8 = 128
  (set `self.PixelSize` (/ (`KismetMathLibrary.Conv_IntToDouble` (`TextureRenderTarget2D.SizeX` (`self.RenderTargetTexture`))) (`KismetMathLibrary.Conv_IntToDouble` (`self.XNum`))))
  ;;[1 1 1] Count Total Pixel of Matrix Canvas
  (bind _output_get (set `self.XYMatrixNum` _returnvalue))
  (`KismetArrayLibrary.Array_Resize` (`self.XYMatrixArray`) _output_get)
  (for _index (range _returnvalue)
    (set `self.IndexCount` _index)
    ;;[1 1 1] Create Matrix Canvas
    (if (not (< (`self.XCount`) (`self.XNum`)))
      (set `self.XCount` 0)
      (`/Engine/EditorBlueprintResources/StandardMacros.IncrementInt` (`self.YCount`)
        (:`  `
          _)))
    (`KismetArrayLibrary.Array_Set` (`self.XYMatrixArray`) (`self.IndexCount`) (`KismetMathLibrary.MakeVector2D` (* (`KismetMathLibrary.Conv_IntToDouble` (`self.XCount`)) _pixelsize) (* _pixelsize (`KismetMathLibrary.Conv_IntToDouble` (`self.YCount`)))))
    (`self.DrawRT` (`|GetArrayItem` (`self.XYMatrixArray`) (`self.IndexCount`)) (`KismetMathLibrary.MakeVector2D` _pixelsize_2 _pixelsize_2) 1.0)
    (`/Engine/EditorBlueprintResources/StandardMacros.IncrementInt` (`self.XCount`))))

(fn `DrawRT`
  (params (Position :type "Vector2D Structure") (Size :type "Vector2D Structure") (Color :type "Float (double-precision)"))
  ;[1 1 1] Draw Normalized Audio Spectrum on Render Target Texture
  (bind (_canvas _size _context) (`KismetRenderingLibrary.BeginDrawCanvasToRenderTarget` (`self.RenderTargetTexture`)))
  (`Canvas.K2_DrawTexture` _canvas null Position Size (0.0 0.0) (1.0 1.0) (make `LinearColor` Color Color Color) "BLEND_Masked" 0.0 (0.5 0.5))
  (`KismetRenderingLibrary.EndDrawCanvasToRenderTarget` _context))

(fn `ModelVisibility`
  (params (ModelArray :type "Array of StaticMeshComponent Object Reference"))
  (for (_array_element _array_index) ModelArray
    (if (== _array_index (`self.ModelIndex`))
      (`SceneComponent.SetVisibility` _array_element true false)
      (else
        (`SceneComponent.SetVisibility` _array_element false false)))))

(fn `PlaySound`
  (params (Sound :type "SoundBase Object Reference"))
  (bind _audio (`self.Audio`))
  (`AudioComponent.Stop` _audio)
  (`AudioComponent.SetSound` _audio null)
  (`AudioComponent.SetSound` _audio Sound)
  (set `self.MusicDuration` (`SoundBase.Duration` Sound))
  (`AudioComponent.Play` (`self.Audio`) 0.0))

(fn `UserConstructionScript`)