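; BP_AccretionDiskTorEmissive is an accretion disk Volwizard Blueprint that derives emissive color from a material's temperature and filter parameters.
; SubwizGetEmissiveColorFromMat reads both vectors from a dynamic material instance, scales the temperature's green channel, max-normalizes the filter and tints it.
; FilterAndTemperatureToColor turns these into chromaticity and luminance, with the filter's peak component multiplied back into the luminance factor.
; Events and construction script only call the parent.
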(event `self.ReceiveBeginPlay`
  (`parent.ReceiveBeginPlay`))

(event `self.ReceiveTick`
  (params (DeltaSeconds :type "Float (single-precision)"))
  (`parent.ReceiveTick` DeltaSeconds))

(fn `SubwizGetEmissiveColorFromMat`
  (params (MID :type "MaterialInstanceDynamic Object Reference") (TemperatureName :type Name) (FilterName :type Name) (Temperaturefactor :type "Float (double-precision)") (FilterFactor :type "LinearColor Structure") (FilterAlphaIsLuminanceFactor :type Boolean))
  (returns (FilteredChromaticity :type "LinearColor Structure") (Luminance :type "Float (double-precision)") (MatTemperature :type "Float (double-precision)") (NormalizedMatFilter :type "LinearColor Structure") (LuminanceFactor :type "Float (double-precision)"))
  (bind (_r _g _b) (break `LinearColor` FilterFactor))
  (bind _returnvalue (`MaterialInstanceDynamic.K2_GetVectorParameterValue` MID TemperatureName))
  (bind _returnvalue_2 (`MaterialInstanceDynamic.K2_GetVectorParameterValue` MID FilterName))
  (bind (_normalizedcolor _maxcomponent) (`/Game/AccretionDisk/Blueprints/BP_Utilities_MLib.ColorMaxNormalize` _returnvalue_2)
    (:`done`
      (bind ((`G` _g_2)) (break `LinearColor` _returnvalue))
      (bind (_filteredchromaticity _luminance _luminancefactor) (`/Game/AccretionDisk/Blueprints/BP_Utilities_MLib.FilterAndTemperatureToColor` (* _normalizedcolor (make `LinearColor` _r _g _b 1.0)) FilterAlphaIsLuminanceFactor (* _g_2 Temperaturefactor)))
      (return _filteredchromaticity _luminance _g_2 _normalizedcolor (* _luminancefactor _maxcomponent)))))

(fn `UserConstructionScript`
  (`parent.UserConstructionScript`))