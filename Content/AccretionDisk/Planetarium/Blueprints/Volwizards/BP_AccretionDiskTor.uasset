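; Accretion disk actor, apparently a volumetric torus, that extends its parent with an optional stellar sphere.
; The construction script sizes the sphere from radius, mesh bounds and geometric scale, or hides it in game without collision.
; A dynamic material instance receives rotation, panning, UV scale, color-filtered emission and a temperature range derived from the actor's temperature.
; A visibility override keeps the sphere in step with the parent and its show flag.
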(event `self.ReceiveBeginPlay`
  (`parent.ReceiveBeginPlay`))

(event `self.ReceiveTick`
  (params (DeltaSeconds :type "Float (single-precision)"))
  (`parent.ReceiveTick` DeltaSeconds))

(fn `SetStellarSphereMaterial`
  (params (StellarMaterial :type "MaterialInterface Object Reference"))
  (returns (StellarMID :type "MaterialInstanceDynamic Object Reference"))
  (`/Engine/EditorBlueprintResources/StandardMacros.IsValid` StellarMaterial
    (:`Is Valid`
      (set `self.StellarSphereMaterial` StellarMaterial)
      (`self.SetStellarSphereMaterialM`)
      (return (`self.StellarSphereMID`)))
    (:`Is Not Valid`
      (return null))))

(fn `SetVisibility`
  (params (IsVisible :type Boolean))
  (returns (_ :type Boolean))
  (bind __ (`parent.SetVisibility` IsVisible))
  (`SceneComponent.SetVisibility` (`self.StellarSphere`) (and __ (`self.bShowStellarSphere`)) false)
  (return __))

(fn `UserConstructionScript`
  (bind _stellarsphere (`self.StellarSphere`))
  (`parent.UserConstructionScript`)
  (if (`self.bShowStellarSphere`)
    (`self.SetStellarSphereScale` (`self.StellarSphereRadius`))
    (`self.SetStellarSphereMaterialM`)
    (else
      (`SceneComponent.SetVisibility` _stellarsphere true false)
      (`SceneComponent.SetHiddenInGame` _stellarsphere true false)
      (`PrimitiveComponent.SetCollisionEnabled` _stellarsphere "NoCollision"))))