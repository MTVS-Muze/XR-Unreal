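; BP_AccretionDisk is an accretion disk Blueprint in the planetarium's Volwizards set, extending a parent wizard class that handles its construction, begin play and tick logic.
; Its own logic is the WizSetLightFunction override, which calls the parent, then copies radius, distance factor and angular speed from the supplied material instance into the light function material, if valid.
; This mapping keeps the light function's disk parameters matched to the disk material.
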(event `self.ReceiveBeginPlay`
  (`parent.ReceiveBeginPlay`))

(event `self.ReceiveTick`
  (params (DeltaSeconds :type "Float (single-precision)"))
  (`parent.ReceiveTick` DeltaSeconds))

(fn `UserConstructionScript`
  (`parent.UserConstructionScript`))

(fn `WizSetLightFunction`
  (params (MID :type "MaterialInstanceDynamic Object Reference"))
  (returns (StepName :type Name))
  (bind _lightfuncmid (`self.lightFuncMID`))
  (`parent.WizSetLightFunction` MID)
  (`|ExecutionSequence`
    (:`then_0`
      (`/Engine/EditorBlueprintResources/StandardMacros.IsValid` _lightfuncmid
        (:`Is Valid`
          (bind _returnvalue (`MaterialInstanceDynamic.K2_GetScalarParameterValue` MID "Radius"))
          (`MaterialInstanceDynamic.SetScalarParameterValue` _lightfuncmid "DiskRadius" _returnvalue)
          (bind _returnvalue_2 (`MaterialInstanceDynamic.K2_GetScalarParameterValue` MID "DistanceFactor"))
          (`MaterialInstanceDynamic.SetScalarParameterValue` _lightfuncmid "DistanceFactor" _returnvalue_2)
          (bind _returnvalue_3 (`MaterialInstanceDynamic.K2_GetScalarParameterValue` MID "AngularSpeedFactor"))
          (`MaterialInstanceDynamic.SetScalarParameterValue` _lightfuncmid "RotationalSpeed" _returnvalue_3))))
    (:`then_1`
      (return "AccretionDisk_SetLightFunction"))))