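; BP_GateTriggerBox is a box-shaped gate trigger that detects when tracked locations pass through its plane and in which direction.
; The construction script sizes PassageVolume and a zero-thickness GatePlane from the extent variables.
; CheckLocation stores each location's side of the ExitArrow plane while inside the volume, returning the sign of any change as passing direction.
; Locations outside the volume register as OutsideLocation, so entering it never counts as passing.
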(fn `AddLocation`
  (params (Location :type "SceneComponent Object Reference"))
  (returns (RelativeLocation :type Integer))
  (bind _passagevolume (`self.PassageVolume`))
  (bind _relativelocation (`parent.AddLocation` Location))
  (return (select `bool` (`KismetMathLibrary.IsPointInBoxWithTransform` (`SceneComponent.K2_GetComponentLocation` Location) (`SceneComponent.K2_GetComponentToWorld` _passagevolume) (`BoxComponent.BoxExtent` _passagevolume)) :`false` (`self.OutsideLocation`) :`true` _relativelocation)))

(fn `CheckLocation`
  (params (Location :type "SceneComponent Object Reference"))
  (returns (PassingDirection :type Integer) (IsTracked :type Boolean))
  (locals (currentRelLocation :type Integer) (passingDir :type Integer) (insidePassageVol :type Boolean))
  (bind _tracks (`self.Tracks`))
  (bind _passagevolume (`self.PassageVolume`))
  (bind (_value _returnvalue) (`BlueprintMapLibrary.Map_Find` _tracks Location))
  (if _returnvalue
    (set `local.insidePassageVol` (`KismetMathLibrary.IsPointInBoxWithTransform` (`SceneComponent.K2_GetComponentLocation` Location) (`SceneComponent.K2_GetComponentToWorld` _passagevolume) (`BoxComponent.BoxExtent` _passagevolume)))
    (bind _output_get (set `local.currentRelLocation` (select `bool` (`local.insidePassageVol`) :`false` (`self.OutsideLocation`) :`true` (`KismetMathLibrary.FTrunc` (`KismetMathLibrary.SignOfFloat` (`/Game/AccretionDisk/Blueprints/BP_Utilities_MLib.DistanceToPlane` Location (`self.ExitArrow`)))))))
    (set `local.passingDir` (select `bool` (and (`local.insidePassageVol`) (!= _value (`self.OutsideLocation`))) :`true` (`KismetMathLibrary.SignOfInteger` (- _output_get _value))))
    (`BlueprintMapLibrary.Map_Add` _tracks (`local.Location`) (`local.currentRelLocation`))
    (return (`local.passingDir`) true)
    (else
      (return 0 false))))

(fn `UserConstructionScript`
  (bind (_x _y) (`KismetMathLibrary.BreakVector2D` (`self.GateExtent`)))
  (bind _returnvalue (`KismetMathLibrary.MakeVector` (`KismetMathLibrary.FMax` (`self.PassageExtent`) 0.01) (`KismetMathLibrary.FMax` _x 0.01) (`KismetMathLibrary.FMax` _y 0.01)))
  (`parent.UserConstructionScript`)
  (`BoxComponent.SetBoxExtent` (`self.PassageVolume`) _returnvalue false)
  (`BoxComponent.SetBoxExtent` (`self.GatePlane`) (`KismetMathLibrary.MakeVector` 0.0 (.y _returnvalue) (.z _returnvalue)) false))