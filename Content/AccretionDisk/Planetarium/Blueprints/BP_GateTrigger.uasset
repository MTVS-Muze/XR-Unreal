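; Gate trigger Blueprint that detects which way tracked locations cross the plane defined by its ExitArrow.
; AddLocation stores the sign of a location's signed distance to that plane in the Tracks map.
; CheckLocation recomputes and stores that side, returning the sign of the change as passing direction, plus whether the location is tracked.
; The event graph is empty, so detection runs only when these functions are called.
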(fn `AddLocation`
  (params (Location :type "SceneComponent Object Reference"))
  (returns (RelativeLocation :type Integer))
  (locals (relLocation :type Integer))
  (bind _output_get (set `local.relLocation` (`KismetMathLibrary.FTrunc` (`KismetMathLibrary.SignOfFloat` (`/Game/AccretionDisk/Blueprints/BP_Utilities_MLib.DistanceToPlane` Location (`self.ExitArrow`))))))
  (`BlueprintMapLibrary.Map_Add` (`self.Tracks`) Location _output_get)
  (return _output_get))

(fn `CheckLocation`
  (params (Location :type "SceneComponent Object Reference"))
  (returns (PassingDirection :type Integer) (IsTracked :type Boolean))
  (locals (currentRelLocation :type Integer) (passingDir :type Integer))
  (bind _tracks (`self.Tracks`))
  (bind (_value _returnvalue) (`BlueprintMapLibrary.Map_Find` _tracks Location))
  (if _returnvalue
    (bind _output_get (set `local.currentRelLocation` (`KismetMathLibrary.FTrunc` (`KismetMathLibrary.SignOfFloat` (`/Game/AccretionDisk/Blueprints/BP_Utilities_MLib.DistanceToPlane` Location (`self.ExitArrow`))))))
    (set `local.passingDir` (`KismetMathLibrary.SignOfInteger` (- _output_get _value)))
    (`BlueprintMapLibrary.Map_Add` _tracks (`local.Location`) (`local.currentRelLocation`))
    (return (`local.passingDir`) true)
    (else
      (return 0 false))))

(fn `UserConstructionScript`)