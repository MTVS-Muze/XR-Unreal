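; Actor that makes a directional light stand in for a point light as seen from an aim point, optionally the player camera.
; Each tick it aims the directional light from the source toward that point and copies color and temperature.
; Intensity converts by light units with inverse-square falloff, smoothstep-fading in with distance across a band derived from the attenuation radius.
; Functions allow swapping the source and switching the output.
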(event `self.ReceiveBeginPlay`
  (bind _binitialized (`self.InitParameters`))
  (`self.SetAim`)
  (`self.SetActorTickEnabled` _binitialized))

(event `self.ReceiveTick`
  (params (DeltaSeconds :type "Float (single-precision)"))
  (bind _aimlocation (`self.UpdateAimLocation`))
  (`self.UpdateParameters` (`self.PointLightComponent`) (`Light.LightComponent` (`self.DirectionalLight`)) _aimlocation))

(fn `InitParameters`
  (returns (bInitialized :type Boolean))
  (bind _pointlight (`self.PointLight`))
  (bind _pointlightcomponent (`self.PointLightComponent`))
  (set `self.bInitialized` false)
  (`|ExecutionSequence`
    (:`then_0`
      (`/Engine/EditorBlueprintResources/StandardMacros.IsValid` (`self.DirectionalLight`)
        (:`Is Valid`
          (`/Engine/EditorBlueprintResources/StandardMacros.IsValid` _pointlight
            (:`Is Valid`
              (bind _output_get (set `self.PointLightComponent` (`self.GetComponentByClass` _pointlight "/Script/Engine.PointLightComponent")))
              (`/Engine/EditorBlueprintResources/StandardMacros.IsValid` _output_get
                (:`Is Valid`
                  (`self.SetFadeLimits` (`LocalLightComponent.AttenuationRadius` _pointlightcomponent))
                  (`self.CopyParameters` _pointlightcomponent (`Light.LightComponent` (`self.DirectionalLight`)))
                  (`SceneComponent.K2_SetWorldRotation` (`self.Arrow`) (`KismetMathLibrary.Conv_VectorToRotator` (`self.direction`)) false true)
                  (set `self.bInitialized` true))))))))
    (:`then_1`
      (return (`self.bInitialized`)))))

(fn `SetPointLightSource`
  (params (NewSource :type "Actor Object Reference"))
  (returns (Source :type "Actor Object Reference") (SourceComponent :type "PointLightComponent Object Reference") (Accepted :type Boolean))
  (locals (isValid :type Boolean))
  (bind _directionallight (`self.DirectionalLight`))
  (set `local.isValid` false)
  (`|ExecutionSequence`
    (:`then_0`
      (bind _output_get (set `self.PointLight` NewSource))
      (`/Engine/EditorBlueprintResources/StandardMacros.IsValid` _output_get
        (:`Is Valid`
          (bind _output_get_2 (set `self.PointLightComponent` (`self.GetComponentByClass` _output_get "/Script/Engine.PointLightComponent")))
          (`/Engine/EditorBlueprintResources/StandardMacros.IsValid` _output_get_2
            (:`Is Valid`
              (`self.SetFadeLimits` (`LocalLightComponent.AttenuationRadius` _output_get_2))
              (set `local.isValid` true)
              (`/Engine/EditorBlueprintResources/StandardMacros.IsValid` _directionallight
                (:`Is Valid`
                  (`self.CopyParameters` (`self.PointLightComponent`) (`Light.LightComponent` _directionallight)))))))))
    (:`then_1`
      (`self.SetTickEnabled` true)
      (return (`self.PointLight`) (`self.PointLightComponent`) (`local.isValid`)))))

(fn `SetTickEnabled`
  (params (NewTickEnabled :type Boolean))
  (returns (TickEnabled :type Boolean))
  (bind _output_get (set `self.bInitialized` (and (`KismetSystemLibrary.IsValid` (`self.DirectionalLight`)) (`KismetSystemLibrary.IsValid` (`self.PointLightComponent`)) (`KismetSystemLibrary.IsValid` (`self.PointLight`)))))
  (bind _returnvalue (and _output_get NewTickEnabled))
  (`self.SetActorTickEnabled` _returnvalue)
  (return _returnvalue))

(fn `SwitchDirectionalLight`
  (params (On :type Boolean) (ForceShutdown :type Boolean :default true))
  (returns (_DirectionalLight :type "DirectionalLight Object Reference"))
  (bind _directionallight (`self.DirectionalLight`))
  (`|ExecutionSequence`
    (:`then_0`
      (`/Engine/EditorBlueprintResources/StandardMacros.IsValid` _directionallight
        (:`Is Valid`
          (if On
            (`/Engine/EditorBlueprintResources/StandardMacros.IsValid` (`self.PointLightComponent`)
              (:`Is Valid`
                (bind _aimlocation (`self.UpdateAimLocation`))
                (`self.UpdateParameters` (`self.PointLightComponent`) (`Light.LightComponent` (`self.DirectionalLight`)) _aimlocation))
              (:`Is Not Valid`
                (if ForceShutdown
                  (`LightComponent.SetIntensity` (`Light.LightComponent` _directionallight) 0.0 :!label _label))))
            (else
              (goto _label))))))
    (:`then_1`
      (return (`self.DirectionalLight`)))))

(fn `UserConstructionScript`
  (set `self.bUseCameraAsAim` (and (not (`KismetSystemLibrary.IsValid` (`self.Aim`))) (`self.bUseCameraAsAim`)))
  (`self.InitParameters`))