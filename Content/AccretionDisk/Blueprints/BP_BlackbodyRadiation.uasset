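; Blackbody radiation helpers for the AccretionDisk content that convert temperature into emitted color and brightness.
; Chromaticity uses fitted rational curves for RGB, with a variant clamping green and blue to non-negative.
; EffectiveRadiance applies a single-exponential Planck-style formula; Color multiplies it by clamped chromaticity and the 683 luminous-efficacy factor, which Luminance pre-folds into its constant.
; Normalization helpers scale colors by their largest channel and also return that maximum.
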(fn `Chromaticity`
  (params (Temperature :type "Float (double-precision)"))
  (returns (Chromaticity :type "LinearColor Structure"))
  (locals (u :type "Vector Structure") (u2 :type "Vector Structure"))
  (bind _temperature (`local.Temperature`))
  (bind _output_get (set `local.u` (* (`KismetMathLibrary.MakeVector` 0.000536 0.001964 0.000941) Temperature)))
  (bind _output_get_2 (set `local.u2` (* _output_get _output_get)))
  (return (make `LinearColor` (+ (/ (+ (.x (`local.u`)) 1.57533) (+ (.x _output_get_2) 0.28664)) 0.638749) (+ (/ (- (.y (`local.u`)) 10.8015) (+ (.y _output_get_2) 6.59002)) 0.971029) (- 2.25398 (/ (+ (* 0.006684 _temperature) 23.3962) (+ (.z _output_get_2) (* 0.001006 _temperature) 10.9068))) 1.0)))

(fn `ChromaticityNonNegative`
  (params (Temperature :type "Float (double-precision)"))
  (returns (Chromaticity :type "LinearColor Structure"))
  (locals (u :type "Vector Structure") (u2 :type "Vector Structure"))
  (bind _temperature (`local.Temperature`))
  (bind _output_get (set `local.u` (* (`KismetMathLibrary.MakeVector` 0.000536 0.001964 0.000941) Temperature)))
  (bind _output_get_2 (set `local.u2` (* _output_get _output_get)))
  (return (make `LinearColor` (+ (/ (+ (.x (`local.u`)) 1.57533) (+ (.x _output_get_2) 0.28664)) 0.638749) (`KismetMathLibrary.FMax` (+ (/ (- (.y (`local.u`)) 10.8015) (+ (.y _output_get_2) 6.59002)) 0.971029)) (`KismetMathLibrary.FMax` (- 2.25398 (/ (+ (* 0.006684 _temperature) 23.3962) (+ (.z _output_get_2) (* 0.001006 _temperature) 10.9068)))) 1.0)))

(fn `Color`
  (params (Temperature :type "Float (double-precision)"))
  (returns (Color :type "LinearColor Structure"))
  (return (* (`self.ChromaticityNonNegative` Temperature) (* (`self.EffectiveRadiance` Temperature) 683.002014))))

(fn `EffectiveRadiance`
  (params (Temperature :type "Float (double-precision)"))
  (returns (Radiance :type "Float (double-precision)"))
  (return (/ 230141696.0 (- (`KismetMathLibrary.Exp` (/ 25724.199219 Temperature)) 1.0))))

(fn `Luminance`
  (params (Temperature :type "Float (double-precision)"))
  (returns (Luminance :type "Float (double-precision)"))
  (return (/ 157187244032.0 (- (`KismetMathLibrary.Exp` (/ 25724.199219 Temperature)) 1.0))))

(fn `NormalizeColorToMaxRGB`
  (params (Color :type "LinearColor Structure"))
  (returns (NormalizedColor :type "LinearColor Structure") (MaxComponent :type "Float (double-precision)"))
  (locals (maxc :type "Float (double-precision)"))
  (bind (_r _g _b _a) (break `LinearColor` Color))
  (bind _output_get (set `local.maxc` (`KismetMathLibrary.FMax` _r _g _b)))
  (if (== _output_get 0.0)
    (return (`local.Color`) 0.0)
    (else
      (return (make `LinearColor` (.x (/ (`KismetMathLibrary.MakeVector` _r _g _b) _output_get)) (.y (/ (`KismetMathLibrary.MakeVector` _r _g _b) _output_get)) (.z (/ (`KismetMathLibrary.MakeVector` _r _g _b) _output_get)) _a) (`local.maxc`)))))

(fn `NormalizedChromaticity`
  (params (Temperature :type "Float (double-precision)"))
  (returns (NormalizedColor :type "LinearColor Structure") (MaxComponent :type "Float (double-precision)"))
  (locals (maxc :type "Float (double-precision)") (clampedChroma :type "Vector Structure"))
  (bind _maxc (`local.maxc`))
  (bind _output_get (set `local.clampedChroma` (`KismetMathLibrary.Conv_LinearColorToVector` (`self.ChromaticityNonNegative` Temperature))))
  (set `local.maxc` (`KismetMathLibrary.FMax` (.x _output_get) (.y _output_get) (.z _output_get)))
  (return (make `LinearColor` (.x (/ (`local.clampedChroma`) _maxc)) (.y (/ (`local.clampedChroma`) _maxc)) (.z (/ (`local.clampedChroma`) _maxc)) 1.0) _maxc))