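; Base actor for volume effects rendered through a post-process material, feeding the actor's transform and tuning into a dynamic material instance.
; Construction creates the instance as the PostProcess blendable, then runs wizard steps: parameter overrides, local-space origin and basis, and geometric scaling.
; Scaling multiplies listed parameters by GeometricScale raised to per-parameter exponents.
; Tick refreshes the local space, enabled only when initialized with all origin and basis parameter names set.
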(event `self.ReceiveBeginPlay`
  (bind (_cantickout _wanttickout) (`self.CheckTickEnabled` (`self.isInitialized`) (not (or (== (`self.OriginName`) "None") (== (`self.BasisXName`) "None") (== (`self.BasisYName`) "None") (== (`self.BasisZName`) "None")))))
  (`self.SetActorTickEnabled` (and _cantickout _wanttickout)))

(event `self.ReceiveTick`
  (params (DeltaSeconds :type "Float (single-precision)"))
  (`self.SetLocalSpace` (`self.VolumeMID`) self))

(fn `CheckTickEnabled`
  (params (CanTickIn :type Boolean) (WantTickIn :type Boolean))
  (returns (CanTickOut :type Boolean) (WantTickOut :type Boolean))
  (return CanTickIn WantTickIn))

(fn `IniConstruction`
  (returns (MID :type "MaterialInstanceDynamic Object Reference") (Initialized :type Boolean))
  (bind _volumemid (`self.VolumeMID`))
  (bind _array (break `WeightedBlendables` (`.WeightedBlendables` (break `PostProcessSettings` (`self.PPSettings`)))))
  (`/Engine/EditorBlueprintResources/StandardMacros.IsValid` (`self.VolumeMaterial`)
    (:`Is Valid`
      (`|ExecutionSequence`
        (:`then_0`
          (bind _returnvalue (`KismetMaterialLibrary.CreateDynamicMaterialInstance` (`self.VolumeMaterial`)))
          (set `self.VolumeMID` _returnvalue))
        (:`then_1`
          (`KismetArrayLibrary.Array_Clear` _array)
          (`KismetArrayLibrary.Array_Add` _array (make `WeightedBlendable` 1.0 (`self.VolumeMID`)))
          (set `PostProcessComponent.Settings` (`self.PPSettings`) (`self.PostProcess`)))
        (:`then_2`
          (set `self.isInitialized` true)
          (return _volumemid true))))
    (:`Is Not Valid`
      (set `self.isInitialized` false)
      (return _volumemid false))))

(fn `RunWizardSteps`
  (params (MID :type "MaterialInstanceDynamic Object Reference") (bReadyIn :type Boolean))
  (returns (bReadyOut :type Boolean))
  ;[0.05 0.05742 0.1] Wizard Steps
  (if bReadyIn
    (`self.WizOverrideMaterialParameters` MID (`self.ScalarOverrides`) (`self.VectorOverrides`))
    (`self.WizSetLocalSpace` MID self)
    (`self.WizApplyGeometricScaling` MID)
    (return true)
    (else
      (return false))))

(fn `SetMaterialVisibility`
  (params (IsVisible :type Boolean))
  (returns (_ :type Boolean))
  (bind _output_get (set `PostProcessComponent.bEnabled` IsVisible (`self.PostProcess`)))
  (return _output_get))

(fn `SetVisibility`
  (params (IsVisible :type Boolean))
  (returns (_ :type Boolean))
  (bind _output_get (set `PostProcessComponent.bEnabled` IsVisible (`self.PostProcess`)))
  (return _output_get))

(fn `UserConstructionScript`
  (bind (_mid _initialized) (`self.IniConstruction`))
  (`self.RunWizardSteps` _mid _initialized))

(fn `WizApplyGeometricScaling`
  (params (MID :type "MaterialInstanceDynamic Object Reference"))
  (returns (StepName :type Name))
  (bind _mid (`local.MID`))
  (bind _mid_2 (`local.MID`))
  (`|ExecutionSequence`
    (:`then_0`
      (bind (_key _value) (`/Game/AccretionDisk/Blueprints/BP_Utilities_MLib.ForEachKeyName` (`self.ScalingScalars`))
        (:`loopBody`
          (bind _returnvalue (`MaterialInstanceDynamic.K2_GetScalarParameterValue` _mid_2 _key))
          (`MaterialInstanceDynamic.SetScalarParameterValue` _mid_2 _key (* _returnvalue (`KismetMathLibrary.MultiplyMultiply_FloatFloat` (`self.GeometricScale`) _value))))))
    (:`then_1`
      (bind (_key_2 _value_2) (`/Game/AccretionDisk/Blueprints/BP_Utilities_MLib.ForEachKeyName` (`self.ScalingVectors`))
        (:`loopBody`
          (bind _returnvalue_2 (`MaterialInstanceDynamic.K2_GetVectorParameterValue` _mid _key_2))
          (`MaterialInstanceDynamic.SetVectorParameterValue` _mid _key_2 (* _returnvalue_2 (`/Game/AccretionDisk/Blueprints/BP_Utilities_MLib.PowVec4` _value_2 (`self.GeometricScale`)))))))
    (:`then_2`
      (return "Base_ApplyGeometricScaling"))))

(fn `WizOverrideMaterialParameters`
  (params (MID :type "MaterialInstanceDynamic Object Reference") (Scalars :type "Map of Name to Float (double-precision)") (Vectors :type "Map of Name to LinearColor Structure"))
  (returns (StepName :type Name))
  (`/Game/AccretionDisk/Blueprints/BP_Utilities_MLib.OverrideParameters` MID Scalars Vectors)
  (return "Base_OverrideMaterialParameters"))

(fn `WizSetLocalSpace`
  (params (MID :type "MaterialInstanceDynamic Object Reference") (LocalSpace :type "Actor Object Reference"))
  (returns (StepName :type Name))
  (`self.SetLocalSpace` MID LocalSpace
    (:`done`
      (return "Base_SetLocalSpace"))))