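; Volumetric "wizard" Blueprint that adds emissive glow to a dynamic material and its matching scene point light color.
; Its setup step reads temperature and color from the material or writes emissive luminance to it, then converts luminance to light intensity from radius and geometric scale.
; Optional Perlin-noise fluctuation of temperature and intensity enables tick and adds flickering emission to the parent's light color.
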(event `self.ReceiveBeginPlay`
  (bind _returnvalue (`KismetMathLibrary.RandomFloat`))
  (`parent.ReceiveBeginPlay`)
  (if (`self.IsActorTickEnabled`)
    (set `self.meanEmissiveColor` (`self.sceneEmissiveColor`))
    (set `self.fluctuationTimeEmissiveTemp` (* (`self.EmissiveTemperatureTimeRate`) _returnvalue))
    (set `self.fluctuationTimeLuminance` (* (`self.EmissiveIntensityTimeRate`) (- 1.0 _returnvalue)))))

(event `self.ReceiveTick`
  (params (DeltaSeconds :type "Float (single-precision)"))
  (`parent.ReceiveTick` DeltaSeconds))

(fn `CheckTickEnabled`
  (params (CanTickIn :type Boolean) (WantTickIn :type Boolean))
  (returns (CanTickOut :type Boolean) (WantTickOut :type Boolean))
  (bind (_cantickout _wanttickout) (`parent.CheckTickEnabled` CanTickIn WantTickIn))
  (return _cantickout (or _wanttickout (`self.bFluctuatingTemperatureChroma`) (`self.bFluctuatingEmissiveIntensity`))))

(fn `ModifySceneLightColor`
  (params (SceneLightColor :type "LinearColor Structure") (DeltaSeconds :type "Float (double-precision)"))
  (returns (ModSceneLightColor :type "LinearColor Structure"))
  (bind _modscenelightcolor (`parent.ModifySceneLightColor` SceneLightColor DeltaSeconds))
  (bind _sceneemissivecolor (`self.EmissiveFluctuation` DeltaSeconds))
  (return (+ _sceneemissivecolor _modscenelightcolor)))

(fn `RunWizardSteps`
  (params (MID :type "MaterialInstanceDynamic Object Reference") (bReadyIn :type Boolean))
  (returns (bReadyOut :type Boolean))
  ;[0.05 0.05742 0.1] Wizard Steps
  (if bReadyIn
    (`self.WizOverrideMaterialParameters` MID (`self.ScalarOverrides`) (`self.VectorOverrides`))
    (`self.WizSetLocalSpace` MID self)
    (`self.WizSetEmissive` MID)
    (`self.WizSetScenePointLight` MID)
    (`self.WizApplyGeometricScaling` MID)
    (return true)
    (else
      (return false))))

(fn `SubwizGetEmissiveColorFromMat`
  (params (MID :type "MaterialInstanceDynamic Object Reference") (TemperatureName :type Name) (FilterName :type Name) (Temperaturefactor :type "Float (double-precision)") (FilterFactor :type "LinearColor Structure") (FilterAlphaIsLuminanceFactor :type Boolean))
  (returns (FilteredChromaticity :type "LinearColor Structure") (Luminance :type "Float (double-precision)") (MatTemperature :type "Float (double-precision)") (NormalizedMatFilter :type "LinearColor Structure") (LuminanceFactor :type "Float (double-precision)"))
  (bind (_filteredchromaticity _luminance _mattemperature _normalizedmatfilter _luminancefactor) (`/Game/AccretionDisk/Blueprints/BP_Utilities_MLib.GetColorFromMatTemperatureAndFilter` MID TemperatureName FilterName Temperaturefactor FilterFactor FilterAlphaIsLuminanceFactor))
  (return _filteredchromaticity _luminance _mattemperature _normalizedmatfilter _luminancefactor))

(fn `SubwizModifySceneLightColor`
  (params (SceneLightColor :type "LinearColor Structure"))
  (returns (ModSceneLightColor :type "LinearColor Structure"))
  (bind _modscenelightcolor (`parent.SubwizModifySceneLightColor` SceneLightColor))
  (return (+ _modscenelightcolor (`self.sceneEmissiveColor`))))

(fn `UserConstructionScript`
  (`parent.UserConstructionScript`)
  (bind _output_get (set `self.bFluctuatingTemperatureChroma` (and (`self.bFluctuatingTemperatureChroma`) (`self.bUseEmissiveTemperature`))))
  (set `self.bFluctuatingTemperatureLuma` (and _output_get (`self.bFluctuatingTemperatureLuma`))))

(fn `WizApplyGeometricScaling`
  (params (MID :type "MaterialInstanceDynamic Object Reference"))
  (returns (StepName :type Name))
  (bind _intensitygeometricscale (`self.IntensityGeometricScale`))
  (`parent.WizApplyGeometricScaling` MID)
  (set `self.LuminanceToIntensityCoeff` (* (`self.LuminanceToIntensityCoeff`) _intensitygeometricscale))
  (set `self.meanEmissiveIntensity` (* (`self.meanEmissiveIntensity`) _intensitygeometricscale))
  (set `self.sceneEmissiveColor` (* (`self.sceneEmissiveColor`) _intensitygeometricscale))
  (return "Emissive_ApplyGeometricScaling"))

(fn `WizSetEmissive`
  (params (MID :type "MaterialInstanceDynamic Object Reference"))
  (returns (StepName :type Name))
  (bind _buseemissivetemperature (`self.bUseEmissiveTemperature`))
  (bind _returnvalue (* (`self.EmissiveTemperature`) (`self.EmissiveTemperatureFactor`)))
  (`|ExecutionSequence`
    (:`then_0`
      (if (`self.bMaterialDrivesBlueprint`)
        (set `self.bUseEmissiveTemperature` true)
        (bind (_filteredchromaticity _luminance _mattemperature _normalizedmatfilter _luminancefactor) (`self.SubwizGetEmissiveColorFromMat` (`local.MID`) (`self.EmissiveTemperatureName`) (`self.EmissiveColorName`) (`self.EmissiveTemperatureFactor`) (`self.EmissiveColorFactor`) (`self.bMatColorAlphaIsLuminanceFactor`)))
        (set `self.sceneEmissiveColor` _filteredchromaticity)
        (set `self.meanEmissiveIntensity` _luminance)
        (set `self.EmissiveTemperature` _mattemperature)
        (bind _output_get (set `self.EmissiveColor` _normalizedmatfilter))
        (setmembers `LinearColor` :`StructRef` _output_get :`A` 1.0)
        (bind _output_get_2 (set `self.LuminanceFactor` _luminancefactor))
        (set `self.ExposureValue` (`KismetMathLibrary.Log` _output_get_2 0.5))
        (else
          (`|ExecutionSequence`
            (:`then_0`
              (if (`self.bUseExposureValue`)
                (set `self.LuminanceFactor` (`KismetMathLibrary.MultiplyMultiply_FloatFloat` 0.5 (`self.ExposureValue`)))
                (else
                  (set `self.ExposureValue` (`KismetMathLibrary.Log` (`self.LuminanceFactor`) 0.5)))))
            (:`then_1`
              (set `self.sceneEmissiveColor` (* (* (`self.EmissiveColor`) (`self.EmissiveColorFactor`)) (select `bool` _buseemissivetemperature :`false` (struct :`R` 1.0 :`G` 1.0 :`B` 1.0 :`A` 1.0) :`true` (`/Game/AccretionDisk/Blueprints/BP_BlackbodyRadiation.ChromaticityNonNegative` _returnvalue))))
              (set `self.meanEmissiveIntensity` (select `bool` _buseemissivetemperature :`false` 1.0 :`true` (`/Game/AccretionDisk/Blueprints/BP_BlackbodyRadiation.Luminance` _returnvalue)))
              (`MaterialInstanceDynamic.SetVectorParameterValue` (`local.MID`) (`self.EmissiveLuminanceName`) (* (* (`self.EmissiveColor`) (select `bool` _buseemissivetemperature :`false` (struct :`R` 1.0 :`G` 1.0 :`B` 1.0 :`A` 1.0) :`true` (`/Game/AccretionDisk/Blueprints/BP_BlackbodyRadiation.Color` (`self.EmissiveTemperature`)))) (`self.LuminanceFactor`))))))))
    (:`then_1`
      (bind _output_get_3 (set `self.LuminanceToIntensityCoeff` (* (`KismetMathLibrary.MultiplyByPi` (`KismetMathLibrary.Square` (`self.EffectiveRadius`))) (`self.LuminanceFactor`) (`self.FakeToSceneConvertionCoeff`))))
      (bind _output_get_4 (set `self.meanEmissiveIntensity` (* _output_get_3 (`self.meanEmissiveIntensity`))))
      (set `self.sceneEmissiveColor` (* (`self.sceneEmissiveColor`) _output_get_4)))
    (:`then_2`
      (return "Emissive_SetEmissive"))))