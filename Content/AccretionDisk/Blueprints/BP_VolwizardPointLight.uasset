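; Volumetric wizard actor that pairs a material-based fake light with a scene point light.
; Wizard steps sync color and intensity in either direction (FakeDrivesScene selects which side leads), then apply geometric scaling to the light.
; Optional exponential attenuation derives from the material's scattering, with Perlin noise varying optical distance on Tick for flicker.
; Pass-through Modify functions serve as hooks to alter light color and scattering.
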(event `self.ReceiveBeginPlay`
  (`parent.ReceiveBeginPlay`)
  (if (`self.IsActorTickEnabled`)
    (set `self.currentAttenuation` (`/Game/AccretionDisk/Blueprints/BP_Utilities_MLib.ExpFloat3` (* (`self.meanScattering`) (* (`self.MeanDistance`) -1.0))))
    (set `self.fluctuationTime` (`KismetMathLibrary.RandomFloatInRange` 0.0 (`self.FluctuationTimeRate`)))))

(event `self.ReceiveTick`
  (params (DeltaSeconds :type "Float (single-precision)"))
  (`parent.ReceiveTick` DeltaSeconds)
  (bind _modscenelightcolor (`self.ModifySceneLightColor` (`self.sceneLightColor`) DeltaSeconds))
  (bind _currentattenuation (`self.AttenuationFluctuation` DeltaSeconds))
  (bind _output_get (set `self.sceneLightFinalColor` (* _currentattenuation _modscenelightcolor)))
  (`self.SetScenePointLight` _output_get))

(fn `CheckTickEnabled`
  (params (CanTickIn :type Boolean) (WantTickIn :type Boolean))
  (returns (CanTickOut :type Boolean) (WantTickOut :type Boolean))
  (bind (_cantickout _wanttickout) (`parent.CheckTickEnabled` CanTickIn WantTickIn))
  (return _cantickout (or _wanttickout (`self.bFluctuatingLightAttenuation`))))

(fn `ModifySceneLightColor`
  (params (SceneLightColor :type "LinearColor Structure") (DeltaSeconds :type "Float (double-precision)"))
  (returns (ModSceneLightColor :type "LinearColor Structure"))
  (return SceneLightColor))

(fn `RunWizardSteps`
  (params (MID :type "MaterialInstanceDynamic Object Reference") (bReadyIn :type Boolean))
  (returns (bReadyOut :type Boolean))
  ;[0.05 0.05742 0.1] Wizard Steps
  (if bReadyIn
    (`self.WizOverrideMaterialParameters` MID (`self.ScalarOverrides`) (`self.VectorOverrides`))
    (`self.WizSetLocalSpace` MID self)
    (`self.WizSetScenePointLight` MID)
    (`self.WizApplyGeometricScaling` MID)
    (return true)
    (else
      (return false))))

(fn `SetVisibility`
  (params (IsVisible :type Boolean))
  (returns (_ :type Boolean))
  (bind __ (`parent.SetVisibility` IsVisible))
  (`SceneComponent.SetVisibility` (`self.ScenePointLight`) __ false)
  (return __))

(fn `SubwizModifyMeanScattering`
  (params (MeanScattering :type "LinearColor Structure"))
  (returns (ModMeanScattering :type "LinearColor Structure"))
  (return MeanScattering))

(fn `SubwizModifySceneLightColor`
  (params (SceneLightColor :type "LinearColor Structure"))
  (returns (ModSceneLightColor :type "LinearColor Structure"))
  (return SceneLightColor))

(fn `UpdateSceneLightColor`
  (returns (Intensity :type "Float (double-precision)") (Color :type "LinearColor Structure"))
  (bind _scenepointlight (`self.ScenePointLight`))
  (`self.SetScenePointLight` (`self.sceneLightFinalColor`))
  (return (`LightComponentBase.Intensity` _scenepointlight) (`LightComponentBase.GetLightColor` _scenepointlight)))

(fn `UserConstructionScript`
  (`parent.UserConstructionScript`))

(fn `WizApplyGeometricScaling`
  (params (MID :type "MaterialInstanceDynamic Object Reference"))
  (returns (StepName :type Name))
  (locals (expScale :type "Float (double-precision)"))
  (bind _scalingvectors (`self.ScalingVectors`))
  (bind _boundingradius (`self.BoundingRadius`))
  (bind (_value _returnvalue) (`BlueprintMapLibrary.Map_Find` _scalingvectors (`self.ColorName`)))
  (bind (_value_2 _returnvalue_2) (`BlueprintMapLibrary.Map_Find` _scalingvectors (`self.IntensityName`)))
  (`parent.WizApplyGeometricScaling` MID)
  (`|ExecutionSequence`
    (:`then_0`
      (if (`self.bFakeDrivesScene`)
        (set `local.expScale` (select `bool` _returnvalue :`true` (`.W` (`KismetMathLibrary.BreakVector4` _value))))
        (else
          (set `local.expScale` (select `bool` _returnvalue_2 :`false` 2.0 :`true` (`KismetMathLibrary.BreakVector4` _value_2)))))
      (set `self.IntensityGeometricScale` (`KismetMathLibrary.MultiplyMultiply_FloatFloat` (`self.GeometricScale`) (`local.expScale`))))
    (:`then_1`
      ;[0.1 0.1 0.1] Scaling is not applied to the already scaled SceneLightColor because SceneLightColor is refreshed in the WizSetScenePointLight step every time before this scaling step
      (bind _output_get (set `self.sceneLightColor` (* (`self.sceneLightColor`) (`self.IntensityGeometricScale`))))
      (`self.SetScenePointLight` (* _output_get (`self.currentAttenuation`)) (select `bool` (`self.bApplyGScalingToBoundingRadius`) :`false` _boundingradius :`true` (* _boundingradius (`KismetMathLibrary.Sqrt` (`self.IntensityGeometricScale`)))) :!via `SetRadiusColorIntensity`)
      (return "PointLight_ApplyGeometricScaling"))))

(fn `WizSetScenePointLight`
  (params (MID :type "MaterialInstanceDynamic Object Reference"))
  (returns (StepName :type Name))
  (bind _busetemperature (`self.bUseTemperature`))
  (`|ExecutionSequence`
    (:`then_0`
      (if (`self.bFakeDrivesScene`)
        (set `self.bUseTemperature` true)
        (bind (_filteredchromaticity _luminance _mattemperature _normalizedmatfilter _luminancefactor) (`/Game/AccretionDisk/Blueprints/BP_Utilities_MLib.GetColorFromMatTemperatureAndFilter` (`local.MID`) (`self.TemperatureName`) (`self.ColorName`) (`self.TemperatureFactor`) (`self.ColorFactor`) (`self.bMatColorAlphaIsIntensityFactor`)))
        (set `self.sceneLightColor` (* _filteredchromaticity (* _luminancefactor (`self.IntensityFactor`) (`self.FakeToSceneConvertionCoeff`))))
        (set `self.Temperature` _mattemperature)
        (bind _output_get (set `self.Color` _normalizedmatfilter))
        (setmembers `LinearColor` :`StructRef` _output_get :`A` 1.0)
        (set `self.Intensity` (* (`self.FakeToSceneConvertionCoeff`) _luminancefactor))
        (else
          (set `self.sceneLightColor` (* (* (* (`self.Color`) (`self.ColorFactor`)) (select `bool` _busetemperature :`false` (struct :`R` 1.0 :`G` 1.0 :`B` 1.0 :`A` 1.0) :`true` (`/Game/AccretionDisk/Blueprints/BP_BlackbodyRadiation.ChromaticityNonNegative` (* (`self.Temperature`) (`self.TemperatureFactor`))))) (* (`self.Intensity`) (`self.IntensityFactor`))))
          (`MaterialInstanceDynamic.SetVectorParameterValue` (`local.MID`) (`self.IntensityName`) (* (* (`self.Color`) (select `bool` _busetemperature :`false` (struct :`R` 1.0 :`G` 1.0 :`B` 1.0 :`A` 1.0) :`true` (`/Game/AccretionDisk/Blueprints/BP_BlackbodyRadiation.ChromaticityNonNegative` (`self.Temperature`)))) (/ (`self.Intensity`) (`self.FakeToSceneConvertionCoeff`)))))))
    (:`then_1`
      (bind _modscenelightcolor (`self.SubwizModifySceneLightColor` (`self.sceneLightColor`)))
      (set `self.sceneLightColor` _modscenelightcolor))
    (:`then_2`
      (if (`self.bSceneLightAttenuation`)
        (bind _meanscattering (`self.GetMeanScatteringFromMID` (`local.MID`) (`self.bMatScatteringAlphaIsFactor`)))
        (bind _modmeanscattering (`self.SubwizModifyMeanScattering` _meanscattering))
        (bind _output_get_2 (set `self.meanScattering` _modmeanscattering))
        (set `self.currentAttenuation` (`/Game/AccretionDisk/Blueprints/BP_Utilities_MLib.ExpFloat3` (* _output_get_2 (* (`self.MeanDistance`) -1.0))))
        (else
          (set `self.bFluctuatingLightAttenuation` false)
          (set `self.currentAttenuation` (struct :`R` 1.0 :`G` 1.0 :`B` 1.0 :`A` 1.0)))))
    (:`then_3`
      (`self.SetScenePointLight` (* (`self.sceneLightColor`) (`self.currentAttenuation`)) (`self.BoundingRadius`) :!via `SetRadiusColorIntensity`)
      (return "PointLight_SetScenePointLight"))))