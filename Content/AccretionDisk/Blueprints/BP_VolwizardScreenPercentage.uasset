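; Volumetric wizard Blueprint for the accretion disk content that adjusts the global screen percentage by camera distance to the actor.
; Radial (spherical) and axial (capsule) regions, optionally derived from material parameters, are set in a wizard step and can be shown as spheres and capsules.
; Each tick it linearly interpolates a percentage per region and takes the lower.
; The result snaps to a grid and is applied via r.ScreenPercentage console command only on change.
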(event `self.ReceiveBeginPlay`
  (`parent.ReceiveBeginPlay`)
  (`self.SetInterpolationCoeffs`))

(event `self.ReceiveTick`
  (params (DeltaSeconds :type "Float (single-precision)"))
  (`parent.ReceiveTick` DeltaSeconds)
  (`self.SetScreenPercentage`))

(fn `CheckTickEnabled`
  (params (CanTickIn :type Boolean) (WantTickIn :type Boolean))
  (returns (CanTickOut :type Boolean) (WantTickOut :type Boolean))
  (bind (_cantickout _wanttickout) (`parent.CheckTickEnabled` CanTickIn WantTickIn))
  (bind (_radialinterpolationenabled _axialinterpolationenabled) (`self.SetInterpolationEnabled`))
  (return _cantickout (or _radialinterpolationenabled _axialinterpolationenabled _wanttickout)))

(fn `RunWizardSteps`
  (params (MID :type "MaterialInstanceDynamic Object Reference") (bReadyIn :type Boolean))
  (returns (bReadyOut :type Boolean))
  ;[0.05 0.05742 0.1] Wizard Steps
  (bind _breadyout (`parent.RunWizardSteps` MID bReadyIn))
  (if _breadyout
    (`self.WizSetInterpolationRegions` MID)
    (return true)
    (else
      (return false))))

(fn `SetNearScreenPercentage`
  (params (Percentage :type "Float (double-precision)") (SetRadial :type Boolean :default true) (SetAxial :type Boolean :default true))
  (returns (RadialPercentage :type "Vector2D Structure") (AxialPercentage :type "Vector2D Structure"))
  (bind _radialpercentage (`self.RadialPercentage`))
  (bind _axialpercentage (`self.AxialPercentage`))
  (bind (_x _y) (`KismetMathLibrary.BreakVector4` (`self.AxialRegion`)))
  (bind (_x_2 _y_2) (`KismetMathLibrary.BreakVector2D` _axialpercentage))
  (bind (_x_3 _y_3) (`KismetMathLibrary.BreakVector2D` (`self.RadialRegion`)))
  (bind (_x_4 _y_4) (`KismetMathLibrary.BreakVector2D` _radialpercentage))
  (set `self.RadialPercentage` (select `bool` (and (`local.SetRadial`) (> Percentage 0.0)) :`false` _radialpercentage :`true` (select `bool` (< _x_3 _y_3) :`false` (`KismetMathLibrary.MakeVector2D` _x_4 Percentage) :`true` (`KismetMathLibrary.MakeVector2D` Percentage _y_4))))
  (set `self.AxialPercentage` (select `bool` (and (`local.SetAxial`) (> Percentage 0.0)) :`false` _axialpercentage :`true` (select `bool` (< _x _y) :`false` (`KismetMathLibrary.MakeVector2D` _x_2 Percentage) :`true` (`KismetMathLibrary.MakeVector2D` Percentage _y_2))))
  (`self.SetInterpolationCoeffs`)
  (`self.SetInterpolationEnabled`)
  (return (`self.RadialPercentage`) (`self.AxialPercentage`)))

(fn `UserConstructionScript`
  (`parent.UserConstructionScript`))

(fn `WizSetInterpolationRegions`
  (params (MID :type "MaterialInstanceDynamic Object Reference"))
  (returns (StepName :type Name))
  (bind _spherea (`self.SphereA`))
  (bind _sphereb (`self.SphereB`))
  (bind _bshowregions (`self.bShowRegions`))
  (bind _bshowregions_2 (`self.bShowRegions`))
  (bind (_x _y) (`KismetMathLibrary.BreakVector2D` (`self.scaledRadialRegion`)))
  (bind (_x_2 _y_2 _z _w) (`KismetMathLibrary.BreakVector4` (`self.scaledAxialRegion`)))
  (bind _returnvalue (/ (- _w _z) 2.0))
  (bind _returnvalue_2 (/ (+ _z _w) 2.0))
  (`self.SetInterpolationRegions` MID)
  (`|ExecutionSequence`
    (:`then_0`
      (`SphereComponent.SetSphereRadius` _spherea _x false)
      (`SceneComponent.SetVisibility` _spherea _bshowregions_2 false)
      (`SphereComponent.SetSphereRadius` _sphereb _y false)
      (`SceneComponent.SetVisibility` _sphereb _bshowregions_2 false))
    (:`then_1`
      (`self.SetCapsule` (`self.CapsuleA`) _returnvalue_2 (+ _returnvalue _x_2) _x_2 _bshowregions)
      (`self.SetCapsule` (`self.CapsuleB`) _returnvalue_2 (+ _returnvalue _y_2) _y_2 _bshowregions))
    (:`then_2`
      (return "ScreenPercentage_SetInterpolationRegions"))))