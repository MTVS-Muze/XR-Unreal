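; Volumetric wizard Blueprint that extends its parent's setup steps by giving the scene point light a dynamic light function material.
; After the parent steps succeed, it creates the material instance, optionally copies the volume's parameters, then applies overrides, light position and scene light color.
; It requests ticking while that instance and a position parameter name exist, updating the light's world position in the material every frame.
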(event `self.ReceiveBeginPlay`
  (`parent.ReceiveBeginPlay`))

(event `self.ReceiveTick`
  (params (DeltaSeconds :type "Float (single-precision)"))
  (bind _lightfuncmid (`self.lightFuncMID`))
  (`parent.ReceiveTick` DeltaSeconds)
  (`/Engine/EditorBlueprintResources/StandardMacros.IsValid` _lightfuncmid
    (:`Is Valid`
      (`MaterialInstanceDynamic.SetVectorParameterValue` _lightfuncmid (`self.LightPositionName`) (`KismetMathLibrary.Conv_VectorToLinearColor` (`SceneComponent.K2_GetComponentLocation` (`self.ScenePointLight`)))))))

(fn `CheckTickEnabled`
  (params (CanTickIn :type Boolean) (WantTickIn :type Boolean))
  (returns (CanTickOut :type Boolean) (WantTickOut :type Boolean))
  (bind (_cantickout _wanttickout) (`parent.CheckTickEnabled` CanTickIn WantTickIn))
  (return _cantickout (or _wanttickout (and (`KismetSystemLibrary.IsValid` (`self.lightFuncMID`)) (!= (`self.LightPositionName`) "None")))))

(fn `RunWizardSteps`
  (params (MID :type "MaterialInstanceDynamic Object Reference") (bReadyIn :type Boolean))
  (returns (bReadyOut :type Boolean))
  ;[0.05 0.05742 0.1] Wizard Steps
  (bind _breadyout (`parent.RunWizardSteps` MID bReadyIn))
  (if _breadyout
    (`self.WizSetLightFunction` MID)
    (return true)
    (else
      (return false))))

(fn `UserConstructionScript`
  (`parent.UserConstructionScript`))

(fn `WizSetLightFunction`
  (params (MID :type "MaterialInstanceDynamic Object Reference"))
  (returns (StepName :type Name))
  (bind _lightfuncmid (`self.lightFuncMID`))
  (`|ExecutionSequence`
    (:`then_0`
      (`/Engine/EditorBlueprintResources/StandardMacros.IsValid` (`self.LightFunction`)
        (:`Is Valid`
          (`|ExecutionSequence`
            (:`then_0`
              (bind _returnvalue (`KismetMaterialLibrary.CreateDynamicMaterialInstance` (`self.LightFunction`)))
              (bind _output_get (set `self.lightFuncMID` _returnvalue))
              (`LightComponent.SetLightFunctionMaterial` (`self.ScenePointLight`) _output_get))
            (:`then_1`
              (if (`self.bHasVolumeParameters`)
                (`MaterialInstanceDynamic.K2_CopyMaterialInstanceParameters` (`self.lightFuncMID`) (`local.MID`) true)
                (set `self.LightPositionName` (`self.OriginName`))))
            (:`then_2`
              (`/Game/AccretionDisk/Blueprints/BP_Utilities_MLib.OverrideParameters` (`self.lightFuncMID`) (`self.ScalarOverridesLF`) (`self.VectorOverridesLF`))
              (`MaterialInstanceDynamic.SetVectorParameterValue` _lightfuncmid (`self.LightPositionName`) (`KismetMathLibrary.Conv_VectorToLinearColor` (`SceneComponent.K2_GetComponentLocation` (`self.ScenePointLight`))))
              (`MaterialInstanceDynamic.SetVectorParameterValue` _lightfuncmid (`self.IntensityName`) (`self.sceneLightColor`)))))))
    (:`then_1`
      (return "LightFunction_SetLightFunction"))))